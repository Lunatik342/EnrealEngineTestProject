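; Charged projectile attack that explodes on impact, with blast size and damage driven by its charge time.
; On a collider hit it destroys itself and spawns an explosion emitter scaled by ExplosionScale and ChargeTime.
; A temporary PlayerAttacksTrigger, scaled the same way but larger, serves as a one-shot area query: overlapping UnitBase actors get a charge-scaled ChangeHP call, then the trigger is destroyed.
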(event OnComponentHit(Collider)
  (params (HitComponent :type Primitive%20Component%20Object%20Reference) (OtherActor :type Actor%20Object%20Reference) (OtherComp :type Primitive%20Component%20Object%20Reference) (NormalImpulse :type Vector :default "0, 0, 0") (Hit :type Hit%20Result%20Structure%20%28by%20ref%29))
  (bind _location (Collision|BreakHitResult Hit))
  (bind _explosionscale (Variables|Default|GetExplosionScale))
  (bind _chargetime (Variables|Default|GetChargeTime))
  (bind _returnvalue (* _explosionscale _chargetime))
  ;[1 1 1] Hit stuff
  (Actor|DestroyActor)
  (Effects|SpawnEmitteratLocation "/Game/StarterContent/Particles/P_Explosion.P_Explosion" _location "0, 0, 0" (* _returnvalue 3.0))
  (bind _returnvalue_2 (Game|SpawnActorfromClass "/Game/Blueprints/SpellsAndAttacks/PlayerAttacksTrigger.PlayerAttacksTrigger_C" (Math|Transform|MakeTransform _location "0, 0, 0" (* _returnvalue 7.0)) "Undefined" 0 0))
  (for _array_element (Collision|GetOverlappingActors _returnvalue_2 0 :!class /Script/Engine.Actor)
    (bind _asunit_base (Utilities|Casting|CastToUnitBase _array_element))
    (Default|ChangeHP _asunit_base (* (+ (Variables|Default|GetChargeTime) 0.7) (Variables|Default|GetProjectileDamage))))
  (Actor|DestroyActor _returnvalue_2))

(event EventBeginPlay)

(fn ConstructionScript)