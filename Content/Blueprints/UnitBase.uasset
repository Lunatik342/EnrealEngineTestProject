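; UnitBase is a unit Blueprint with character movement that provides health handling and a configurable movement speed.
; BeginPlay copies MovementSpeed into the movement component's max walk speed, and AnyDamage passes damage to ChangeHP.
; ChangeHP subtracts the amount, keeps HP between zero and MaxHP, and calls the empty UnitDied event at zero.
; ChangeMaxHP adds to MaxHP, printing an error and resetting it to one if the result is non-positive.
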(event Custom|UnitDied)

(event EventBeginPlay
  (Variables|/Script/Engine.CharacterMovementComponent|SetMaxWalkSpeed (Variables|Character|GetCharacterMovement) (Variables|Default|GetMovementSpeed)))

(event Game|Damage|EventAnyDamage
  (params (Damage :type Float%20%28single-precision%29) (DamageType :type Damage%20Type%20Object%20Reference) (InstigatedBy :type Controller%20Object%20Reference) (DamageCauser :type Actor%20Object%20Reference))
  (CallFunction|ChangeHP Damage))

(fn ConstructionScript)

(fn ChangeHP
  (params (Amount :type Float%20%28single-precision%29))
  (if (> (- (Variables|Default|GetCurrentHP) Amount) (Variables|Default|GetMaxHP))
    (Variables|Default|SetCurrentHP (Variables|Default|GetMaxHP))
    (elif (<= (- (Variables|Default|GetCurrentHP) Amount) 0.0)
      (Variables|Default|SetCurrentHP 0.0)
      (CallFunction|UnitDied)
      (else
        (Variables|Default|SetCurrentHP (- (Variables|Default|GetCurrentHP) Amount)))))
  (return (Variables|Default|GetCurrentHP)))

(fn ChangeMaxHP
  (params (Amount :type Float%20%28single-precision%29))
  (if (<= (+ Amount (Variables|Default|GetMaxHP)) 0.0)
    (Development|PrintText "ERRORRRRRRRRRRRRRRRRRRRRRR")
    (Variables|Default|SetMaxHP 1.0)
    (else
      (bind _output_get (Variables|Default|SetMaxHP (+ Amount (Variables|Default|GetMaxHP))))))
  (return _output_get))